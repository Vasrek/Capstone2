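; Enemy AI character that searches for BP_MyCharacter and shoots BP_BallProjectile at them.
; AI Perception toggles Tick between moving to random navmesh points, later centred on the last sensed location, and stopping to fire after random delays.
; A resettable DoOnce gates picking new search points.
; Death plays a random montage, calls death dispatchers, disables capsule collision and destroys the actor after a delay.
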(event `self.ReceiveBeginPlay`
  (bind _randomlocation (`NavigationSystemV1.K2_GetRandomLocationInNavigableRadius` (`self.K2_GetActorLocation`) 5000.0 null null))
  (set `self.LocationToSearch` _randomlocation)
  (bind _asbp_my_character (cast `/Game/Blueprints/BP_MyCharacter` (`GameplayStatics.GetPlayerCharacter` 0)))
  (set `self.PlayerReference` _asbp_my_character))

(event `self.ReceiveTick`
  (params (DeltaSeconds :type "Float (single-precision)"))
  (if (`self.IsAlive?`)
    (if (`self.CanSeeThePlayer`)
      (`MovementComponent.StopMovementImmediately` (`self.CharacterMovement`))
      (`KismetSystemLibrary.Delay` (`KismetMathLibrary.RandomFloatInRange` 0.25 1.5))
      (`self.Fire`)
      (else
        (`|AIMoveTo` self (`self.LocationToSearch`) null
          (:`OnSuccess`
            (`self.ResetChooseRandomLocToSearchThePlayer`)
            (`KismetSystemLibrary.Delay` 2.0)
            (`self.ChooseRandomLocToSearchThePlayer`)))))
    (else
      (`MovementComponent.StopMovementImmediately` (`self.CharacterMovement`)))))

(event `self.AIPerception.OnTargetPerceptionUpdated`
  (params (Actor :type "Actor Object Reference") (Stimulus :type "AIStimulus Structure"))
  (if Stimulus_bSuccessfullySensed
    (bind _asbp_my_character (cast `/Game/Blueprints/BP_MyCharacter` Actor))
    (set `self.PlayerRef` _asbp_my_character)
    (set `self.PlayerLocation` Stimulus_StimulusLocation)
    (set `self.CanSeeThePlayer` true)
    (else
      (set `self.LastPlayerLocation` Stimulus_StimulusLocation)
      (set `self.CanSeeThePlayer` false)
      (`/Engine/EditorBlueprintResources/StandardMacros.DoOnce` false :!label _label
        (:`Completed`
          (bind _randomlocation (`NavigationSystemV1.K2_GetRandomLocationInNavigableRadius` (`self.LastPlayerLocation`) 1000.0 null null))
          (set `self.LocationToSearch` _randomlocation))))))

(event `ChooseRandomLocToSearchThePlayer`
  (goto _label))

(event `ResetChooseRandomLocToSearchThePlayer`
  (goto _label :!via `Reset`))

(event `Fire`
  (bind (_returnvalue_location _returnvalue_rotation) (`KismetMathLibrary.BreakTransform` (`SceneComponent.K2_GetComponentToWorld` (`self.BallSpawner`))))
  (if (and (`self.IsAlive?`) (`/Game/Blueprints/BP_MyCharacter.isAlive?` (`self.PlayerReference`)))
    (`self.K2_SetActorRotation` (`KismetMathLibrary.FindLookAtRotation` (`SceneComponent.K2_GetComponentLocation` (`self.ChildActor`)) (`self.K2_GetActorLocation` (`GameplayStatics.GetPlayerCharacter` 0))))
    (`KismetSystemLibrary.LineTraceSingle` (`self.K2_GetActorLocation`) (`self.K2_GetActorLocation` (`GameplayStatics.GetPlayerCharacter` 0)) "TraceTypeQuery1")
    (`|SpawnActorFromClass` "/Game/Blueprints/BP_BallProjectile.BP_BallProjectile_C" (`KismetMathLibrary.MakeTransform` _returnvalue_location _returnvalue_rotation) "Undefined" "OverrideRootScale" null null)
    (`GameplayStatics.PlaySoundAtLocation` "/Game/FPWeapon/Audio/FirstPersonTemplateWeaponFire02.FirstPersonTemplateWeaponFire02" (0.0 0.0 0.0) (struct) 1.0 1.0 0.0 null null null null) ; Play firing sound
    (`self.PlayAnimMontage` "/Game/Animations/IA/FPSAnimation/AM_Fire.AM_Fire")))

(event `Death`
  (if (`self.IsAlive?`)
    (set `self.IsAlive?` false)
    (`self.PlayAnimMontage` (`KismetArrayLibrary.Array_Random` (`self.DeathAnimMontage`)))
    (`self.DeathEventDispatchers`)
    (`PrimitiveComponent.SetCollisionEnabled` (`self.CapsuleComponent`) "NoCollision")
    (`KismetSystemLibrary.Delay` (`KismetMathLibrary.RandomFloatInRange` 5.0 10.0))
    (`self.K2_DestroyActor`)))

(fn `MoveIAToSpecificLoc`)

(fn `UserConstructionScript`)