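; BP_GameManager runs endless, growing waves of BP_MyIA enemies with start and clear sounds.
; After a startup delay, SpawnIA spawns enemies at the level's TargetPoints by loop index, skipping invalid entries.
; After each spawn and short Delay, it binds DecreaseIARemaining to every BP_MyIA's death dispatcher.
; When the counter, set from the requested count rather than actual spawns, reaches zero, GoToNextWave waits, enlarges the wave and respawns.
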(event `self.ReceiveBeginPlay`
  (bind _outactors (`GameplayStatics.GetAllActorsOfClass` "/Script/Engine.TargetPoint"))
  (set `self.IASpawners` _outactors)
  (`KismetSystemLibrary.Delay` 5.0)
  (`self.SpawnIA`)
  (set `self.WaveNB` 1))

(event `SpawnIA`
  (bind _nbiatospawn (`self.NbIAToSpawn`))
  (`GameplayStatics.PlaySound2D` "/Game/SFX/NextWave.NextWave" 1.0 1.0 0.0 null null)
  (for _index (range (+ _nbiatospawn 1))
    (bind _output (`|GetArrayItem` (`self.IASpawners`) _index))
    (`/Engine/EditorBlueprintResources/StandardMacros.IsValid` _output
      (:`Is Valid`
        (`|SpawnActorFromClass` "/Game/Blueprints/BP_MyIA.BP_MyIA_C" (`self.GetTransform` _output) "Undefined" "OverrideRootScale" null null)
        (`KismetSystemLibrary.Delay` 0.2)
        (bind _outactors (`GameplayStatics.GetAllActorsOfClass` "/Game/Blueprints/BP_MyIA.BP_MyIA_C"))
        (for _array_element _outactors
          (add `/Game/Blueprints/BP_MyIA.DeathEventDispatchers` _array_element (delegate `DecreaseIARemaining`))))))
  (set `self.NbIARemaining` (+ _nbiatospawn 1)))

(event `DecreaseIARemaining`
  (bind _result (`/Engine/EditorBlueprintResources/StandardMacros.DecrementInt` (`self.NbIARemaining`))
    (:`  `
      (if (<= _result 0)
        (set `self.NbIARemaining` 0)
        (`self.GoToNextWave`)))))

(event `GoToNextWave`
  (`GameplayStatics.PlaySound2D` "/Game/SFX/WaveClear.WaveClear" 1.0 1.0 0.0 null null)
  (`KismetSystemLibrary.Delay` 5.0)
  (set `self.NbIAToSpawn` (+ (`self.NbIAToSpawn`) 2))
  (`/Engine/EditorBlueprintResources/StandardMacros.IncrementInt` (`self.WaveNB`)
    (:`  `
      (`self.SpawnIA`))))

(fn `UserConstructionScript`)