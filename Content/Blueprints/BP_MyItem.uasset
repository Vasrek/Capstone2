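; BP_MyItem is a respawning pickup that grants health or ammo, chosen by its ItemList value, when BP_MyCharacter overlaps its box.
; Each pickup plays a sound and runs ResetBox, which disables collision and hides the Niagara effect until a cooldown delay ends.
; GoUp and GoDown define a timer-driven VInterpTo bobbing loop, but its setup is disconnected from BeginPlay, so it never starts.
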(event `self.ReceiveBeginPlay`)

(event `self.Box.OnComponentBeginOverlap`
  (params (OverlappedComponent :type "PrimitiveComponent Object Reference") (OtherActor :type "Actor Object Reference") (OtherComp :type "PrimitiveComponent Object Reference") (OtherBodyIndex :type Integer) (bFromSweep :type Boolean) (SweepResult :type "HitResult Structure (by ref)"))
  (bind _asbp_my_character (cast `/Game/Blueprints/BP_MyCharacter` OtherActor))
  (switch `/Game/Blueprints/E_ItemList` (`self.ItemList`)
    (:`NewEnumerator0`
      (`/Game/Blueprints/BP_MyCharacter.IncreaseHealth` _asbp_my_character (`self.HealthValueToAdd`)))
    (:`NewEnumerator1`
      (`/Game/Blueprints/BP_MyCharacter.IncreaseAmmo` _asbp_my_character (`self.AmmoToAdd`))))
  (`self.ResetBox`)
  (`GameplayStatics.PlaySound2D` "/Game/SFX/pickup.pickup" 1.0 1.0 0.0 null null))

(event `ResetBox`
  (`PrimitiveComponent.SetCollisionEnabled` (`self.Box`) "NoCollision")
  (`SceneComponent.SetHiddenInGame` (`self.Niagara`) true false)
  (`KismetSystemLibrary.Delay` (`self.CooldownResetBox`))
  (`PrimitiveComponent.SetCollisionEnabled` (`self.Box`) "QueryAndPhysics")
  (`SceneComponent.SetHiddenInGame` (`self.Niagara`) false false))

(fn `GoDown`
  (bind _defaultlocation (`self.DefaultLocation`))
  (bind _returnvalue (`KismetMathLibrary.VInterpTo` (`self.K2_GetActorLocation`) _defaultlocation (`GameplayStatics.GetWorldDeltaSeconds`) (`self.InterpSpeed`)))
  (`self.K2_SetActorLocation` _returnvalue)
  (if (== _returnvalue _defaultlocation :`ErrorTolerance` 1.0)
    (`KismetSystemLibrary.K2_ClearTimer` null "GoDown")
    (`KismetSystemLibrary.K2_SetTimer` null "GoUp" 0.01 true)))

(fn `GoUp`
  (bind _locationtogo (`self.LocationToGo`))
  (bind _returnvalue (`KismetMathLibrary.VInterpTo` (`self.K2_GetActorLocation`) _locationtogo (`GameplayStatics.GetWorldDeltaSeconds`) (`self.InterpSpeed`)))
  (`self.K2_SetActorLocation` _returnvalue)
  (if (== _returnvalue _locationtogo :`ErrorTolerance` 1.0)
    (`KismetSystemLibrary.K2_ClearTimer` null "GoUp")
    (`KismetSystemLibrary.K2_SetTimer` null "GoDown" 0.01 true)))

(fn `UserConstructionScript`)